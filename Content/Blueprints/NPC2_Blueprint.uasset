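; NPC2 is a side-scroller enemy that patrols between two fixed points and chases the player on sight.
; Pawn sensing speeds it up via AIMoveTo if the player is visible, and a retriggerable delay drops the chase.
; Reaching the player freezes both characters and quits the game.
; Tick drives patrol and the death physics with teleport, while an overlap trigger flags the player as near.
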(event `self.PawnSensing.OnSeePawn`
  (params (Pawn :type "Pawn Object Reference"))
  ;[1 1 1] Jakis syf
  (bind _asside_scroller_character (cast `/Game/SideScrollerBP/Blueprints/SideScrollerCharacter` Pawn))
  (set `/Game/SideScrollerBP/Blueprints/SideScrollerCharacter.Hidden` false _asside_scroller_character)
  (if (`/Game/SideScrollerBP/Blueprints/SideScrollerCharacter.isVisible` _asside_scroller_character)
    (set `self.triggered` true)
    (`KismetSystemLibrary.PrintString` "JESTEŚ WIDOCZNY")
    (set `CharacterMovementComponent.MaxWalkSpeed` 450.0 (`self.CharacterMovement`))
    (`|AIMoveTo` self (0.0 0.0 0.0) _asside_scroller_character 5.0
      (:`then`
        (bind _output_get (set `self.delay` 10.0))
        (`KismetSystemLibrary.RetriggerableDelay` _output_get)
        (`KismetSystemLibrary.PrintString` "ZGUBIONO POŚCIG \n \nHUEHUEHUEHUEHUE")
        (set `self.triggered` false)
        (set `/Game/SideScrollerBP/Blueprints/SideScrollerCharacter.Hidden` true _asside_scroller_character))
      (:`OnSuccess`
        (`KismetSystemLibrary.PrintString` "YOU DIED" true true (struct :`G` 0.66 :`B` 1.0 :`A` 1.0) 200.0)
        (`CharacterMovementComponent.DisableMovement` (`self.CharacterMovement`))
        (`CharacterMovementComponent.DisableMovement` (`Character.CharacterMovement` (`GameplayStatics.GetPlayerCharacter` 0)))
        (`KismetSystemLibrary.Delay` 5.0)
        (`KismetSystemLibrary.QuitGame` null "Quit")))))

(event `self.ReceiveTick`
  (params (DeltaSeconds :type "Float (single-precision)"))
  ;[1 1 1] Ragdoll
  (if (`self.isDeadNPC2`)
    (`PrimitiveComponent.SetSimulatePhysics` (`self.Mesh`) true)
    (`PrimitiveComponent.SetSimulatePhysics` (`self.CapsuleComponent`) true)
    (`CharacterMovementComponent.DisableMovement` (`self.CharacterMovement`))
    (`self.K2_TeleportTo` (20.0 0.0 0.0) (struct))
    (else
      ;[1 1 1] Jakis syf
      (if (not (`self.triggered`))
        (set `CharacterMovementComponent.MaxWalkSpeed` 100.0 (`self.CharacterMovement`))
        (if (`self.left`) :!label _label
          (`|AIMoveTo` self (1180.0 -2300.0 110.0) null 5.0 true
            (:`OnSuccess`
              (`KismetSystemLibrary.Delay` 1.5)
              (set `self.left` false)
              (goto _label)))
          (else
            (`|AIMoveTo` self (1180.0 -3400.0 110.0) null 5.0 true
              (:`OnSuccess`
                (`KismetSystemLibrary.Delay` 1.5)
                (set `self.left` true)
                (goto _label)))))))))

(event `self.NearTrigger.OnComponentBeginOverlap`
  (params (OverlappedComponent :type "PrimitiveComponent Object Reference") (OtherActor :type "Actor Object Reference") (OtherComp :type "PrimitiveComponent Object Reference") (OtherBodyIndex :type Integer) (bFromSweep :type Boolean) (SweepResult :type "HitResult Structure (by ref)"))
  ;[1 1 1] NEAR TRIGGER
  (bind _asside_scroller_character (cast `/Game/SideScrollerBP/Blueprints/SideScrollerCharacter` (`GameplayStatics.GetPlayerCharacter` 0))
    (:`then`
      (set `/Game/SideScrollerBP/Blueprints/SideScrollerCharacter.nearNPC` true _asside_scroller_character))
    (:`CastFailed`
      (set `/Game/SideScrollerBP/Blueprints/SideScrollerCharacter.nearNPC` false _asside_scroller_character))))

(fn `UserConstructionScript`
  (`parent.UserConstructionScript`))